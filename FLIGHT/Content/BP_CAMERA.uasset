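; Shared multiplayer camera that every player controller views through, framing all player pawns from the game mode's list.
; After a short startup delay, a looping timer eases the camera toward the average position of the valid pawns.
; Spring arm length follows the clamped largest distance between players plus the highest measured speed, zooming out as they spread or speed up.
; Events drop destroyed players from the list and pause updates when all are gone.
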(event `FixCamera`
  (params (`Which player destroyed` :type "/Game/Lander/Lander Object Reference"))
  (bind _player_ref (`self.Player_ref`))
  (`/Engine/EditorBlueprintResources/StandardMacros.IncrementInt` (`self.PlayerDestroyed`)
    (:`  `
      (for (_array_element _array_index) (`self.Player_ref`)
        (if (== _array_element `Which player destroyed`)
          (`KismetArrayLibrary.Array_RemoveItem` _player_ref (`|GetArrayItem` _player_ref _array_index)))))))

(event `self.ReceiveBeginPlay`
  (`KismetSystemLibrary.Delay` 1.2)
  (`self.ClassSetup`)
  (`KismetSystemLibrary.K2_SetTimer` null "UpdateCamera" 0.01 true))

(event `UpdateCamera`
  (set `self.PlayerCount` (`KismetArrayLibrary.Array_Length` (`self.Player_ref`)))
  (`self.SetCameraPOSP4`)
  (`self.SetSpringArmLength`))

(event `AllPlayersDestroyed`
  (`KismetSystemLibrary.K2_PauseTimer` null "UpdateCamera"))

(fn `ClassSetup`
  (bind _asdefault_gm (cast `/Game/Blueprints/Default_GM` (`GameplayStatics.GetGameMode`)))
  (bind _output_get (set `self.BP_GAMEMODE` _asdefault_gm))
  (set `self.Player_ref` (`/Game/Blueprints/Default_GM.PlayerPawns` _output_get))
  (bind _outactors (`GameplayStatics.GetAllActorsOfClass` "/Script/Engine.PlayerController"))
  (`PlayerController.SetViewTargetWithBlend` _outactors self 0.0 "VTBlend_Linear" 0.0 false)
  (for (_array_element _array_index) (`self.Player_ref`)
    (switch `int` _array_index
      (:`0`
        (set `self.P1` _array_element))
      (:`1`
        (set `self.P2` _array_element))
      (:`2`
        (set `self.P3` _array_element))
      (:`3`
        (set `self.P4` _array_element)))))

(fn `SetCameraPOSP4`
  (locals (ActiveLanders :type "Array of /Game/Lander/Lander Object Reference") (Locations :type "Array of Vector Structure"))
  (for _array_element (`self.Player_ref`)
    (`/Engine/EditorBlueprintResources/StandardMacros.IsValid` _array_element
      (:`Is Valid`
        (`KismetArrayLibrary.Array_Add` (`local.Locations`) (`self.K2_GetActorLocation` _array_element)))))
  (set `self.TargetPOS` (`KismetMathLibrary.GetVectorArrayAverage` (`local.Locations`)))
  (`self.K2_SetActorLocation` (`KismetMathLibrary.VInterpTo` (`self.PreviousPOS`) (`self.TargetPOS`) (`GameplayStatics.GetWorldDeltaSeconds`) (`self.INterpSpeed`)))
  (bind _output_get (set `self.PreviousPOS` (`self.K2_GetActorLocation`)))
  (set `self.Altitude` (.z _output_get)))

(fn `SetSpringArmLength`
  (locals (Distances :type "Array of Float (double-precision)") (Velocities :type "Array of Float (double-precision)"))
  (bind _player_ref (`self.Player_ref`))
  (bind _returnvalue (`KismetArrayLibrary.Array_Length` _player_ref))
  (for _index (range (+ (- _returnvalue 2) 1))
    (bind _output (`|GetArrayItem` _player_ref _index))
    (`/Engine/EditorBlueprintResources/StandardMacros.IsValid` _output
      (:`Is Valid`
        (for _index_2 (range (+ _index 1) _returnvalue)
          (bind _output_2 (`|GetArrayItem` (`self.Player_ref`) _index_2))
          (`/Engine/EditorBlueprintResources/StandardMacros.IsValid` _output_2
            (:`Is Valid`
              (`KismetArrayLibrary.Array_Add` (`local.Distances`) (`self.GetDistanceTo` _output _output_2)))))
        (`KismetArrayLibrary.Array_Add` (`local.Velocities`) (`KismetMathLibrary.VSize` (`self.GetVelocity` _output))))))
  (set `SpringArmComponent.TargetArmLength` (+ (`KismetMathLibrary.FClamp` (`.MaxValue` (`KismetMathLibrary.MaxOfFloatArray` (`local.Distances`))) (`self.MinArmLength`) (`self.MaxArmLength`)) (`.MaxValue` (`KismetMathLibrary.MaxOfFloatArray` (`local.Velocities`)))) (`self.SpringArm`)))

(fn `UserConstructionScript`)