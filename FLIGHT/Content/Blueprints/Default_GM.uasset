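; Game mode that sets up competitive local-multiplayer lander rounds.
; StartCompetitiveRound stores the player and round limits and opens the map; once loading finishes, SpawnPlayers creates local players, possessing a Lander spawned at each PlayerStart tagged with the player index.
; It then adds each controller's HUD, incrementing the round number inside that per-player loop.
; A landing counter feeds RoundEnd, which only gathers player states when the count equals the Landers present.
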(event `self.ReceiveBeginPlay`)

(event `StartCompetitiveRound`
  (params (MapName :type Name) (`Number Of Players` :type Integer) (`Number of Rounds` :type Integer) (OtherSettings :type Boolean))
  (set `self.MaxNumberOfRounds` `Number of Rounds`)
  (set `self.Max Players` `Number Of Players`)
  (`GameplayStatics.OpenLevel` MapName))

(event `LevelFinished Loading`
  (`self.SpawnPlayers`)
  (for _index (range (`self.Max Players`))
    (bind _aslander_pc (cast `/Game/Lander/Lander_PC` (`GameplayStatics.GetPlayerController` _index)))
    (`/Game/Lander/Lander_PC.AddHUD To Screens` _aslander_pc)
    (`/Engine/EditorBlueprintResources/StandardMacros.IncrementInt` (`self.RoundNumber`))))

(event `PlayerLandingSuccessfuly`
  (set `self.PlayersLanded` (+ (`self.PlayersLanded`) 1)))

(event `RoundEnd`
  ;[1 1 1] All players have either landed, or are dead
  (bind _outactors (`GameplayStatics.GetAllActorsOfClass` "/Game/Lander/Lander.Lander_C"))
  (if (== (`KismetArrayLibrary.Array_Length` _outactors) (`self.PlayersLanded`))
    (for _array_element (`self.PlayerControllers`)
      (bind _ascompetitive_player_state (cast `/Game/Blueprints/Competitive_PlayerState` (`Controller.PlayerState` _array_element)))
      (`KismetArrayLibrary.Array_Add` (`self.States`) _ascompetitive_player_state))))

(fn `SpawnPlayers`
  (locals (PlayerStarts :type "Array of PlayerStart Object Reference"))
  (bind _index (`self.Index`))
  (bind _returnvalue (`GameplayStatics.GetPlayerController` _index))
  (bind _outactors (`GameplayStatics.GetAllActorsOfClass` "/Script/Engine.PlayerStart"))
  (set `local.PlayerStarts` _outactors)
  (for _index_2 (range (`self.Max Players`))
    (set `self.Index` _index_2)
    (for _array_element (`local.PlayerStarts`)
      (if (== (`PlayerStart.PlayerStartTag` _array_element) (`KismetStringLibrary.Conv_StringToName` (`KismetStringLibrary.Conv_IntToString` (`self.Index`))))
        (`GameplayStatics.CreatePlayer` (`self.Index`))
        (bind _returnvalue_2 (`|SpawnActorFromClass` "/Game/Lander/Lander.Lander_C" (`self.GetTransform` _array_element) "AdjustIfPossibleButAlwaysSpawn" "OverrideRootScale" null null))
        (bind _aslander_pc (cast `/Game/Lander/Lander_PC` _returnvalue))
        (set `/Game/Lander/Lander_PC.PlayerID` _index _aslander_pc)
        (`Controller.Possess` _returnvalue _returnvalue_2)
        (`WidgetBlueprintLibrary.SetInputMode_GameOnly` _returnvalue)
        (`/Game/Lander/Lander.SetPlayerOwner` _returnvalue_2 _index)
        (`KismetArrayLibrary.Array_AddUnique` (`self.PlayerPawns`) _returnvalue_2))))
  (bind _outactors_2 (`GameplayStatics.GetAllActorsOfClass` "/Game/Lander/Lander_PC.Lander_PC_C"))
  (set `self.PlayerControllers` _outactors_2))

(fn `UserConstructionScript`)