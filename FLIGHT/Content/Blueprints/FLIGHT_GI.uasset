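; FLIGHT game instance that keeps competitive match state across level loads and handles returning to or quitting from the main menu.
; StartCompetitiveRound stores level, player count, round count and settings, then opens the level.
; StartNewRround increments the round and replays those settings unless the limit is reached.
; It also stores per-player sprites and accumulates score totals, while GameOver is an empty stub.
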(event `Return To Main Menu`
  (`WidgetLayoutLibrary.RemoveAllWidgets`)
  (bind _returnvalue (`GameplayStatics.GetCurrentLevelName` true))
  (if (`KismetStringLibrary.EqualEqual_StrStr` _returnvalue "Main")
    (`KismetSystemLibrary.QuitGame` null "Quit")
    (else
      (`GameplayStatics.OpenLevel` "Main"))))

(event `StartCompetitiveRound`
  (params (Level :type Name) (`Num Players` :type Integer) (`Num Rounds` :type Integer) (AdvancesSettings :type "/Game/Blueprints/GameSettings_struct Structure"))
  ;[1 1 1] Settings will persist between level resets... Can be changed in through main menu
  (set `self.MaxNumberOfRounds` `Num Rounds`)
  (set `self.Max Players` `Num Players`)
  (set `self.InstanceSettings` AdvancesSettings)
  (set `self.LevelName` Level)
  (bind _returnvalue (`GameplayStatics.GetCurrentLevelName` true))
  (if (`KismetStringLibrary.EqualEqual_StrStr` _returnvalue (`KismetStringLibrary.Conv_NameToString` (`self.LevelName`)))
    _
    (else
      _))
  (`GameplayStatics.OpenLevel` (`self.LevelName`)))

(event `Add PlayerSprite`
  (params (`Sprite to Add` :type "PaperSprite Object Reference") (Index :type Integer))
  ;[1 1 1] Modify Player Sprites: Player sprites remain constant until changed in GameSetupScreen Widget
  (`KismetArrayLibrary.Array_Set` (`self.PlayerSprites`) Index `Sprite to Add` true))

(event `PlayerTotals`
  (params (Player :type Integer) (RoundScore :type Integer))
  (bind _totalplayerscores (`self.TotalPlayerScores`))
  (bind _totalplayerscores_2 (`self.TotalPlayerScores`))
  (if (`KismetArrayLibrary.Array_IsValidIndex` _totalplayerscores Player)
    (`KismetArrayLibrary.Array_Set` _totalplayerscores_2 Player (+ RoundScore (`|GetArrayItem` _totalplayerscores Player)) true)
    (else
      (`KismetArrayLibrary.Array_Add` _totalplayerscores_2 RoundScore))))

(event `Start New Rround`
  (bind _currentroundnumber (`self.CurrentRoundNumber`))
  ;[1 1 1] Start a new round with the same settings
  (`/Engine/EditorBlueprintResources/StandardMacros.IncrementInt` _currentroundnumber
    (:`  `
      (if (not (== _currentroundnumber (`self.MaxNumberOfRounds`)))
        (`self.StartCompetitiveRound` (`self.LevelName`) (`self.Max Players`) (`self.MaxNumberOfRounds`) (`self.InstanceSettings`))))))

(event `Game Over`
  ;[1 1 1] Played Max Rounds, Show totals and winner, then return to main menu
)