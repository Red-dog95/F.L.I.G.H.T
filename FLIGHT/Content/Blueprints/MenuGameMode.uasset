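; MenuGameMode is a menu game mode that sets up local players and their controllers for multiplayer on one machine.
; On BeginPlay it creates a local player with a controller for each slot up to MaxPlayers, then caches all PlayerControllers in PCArray.
; CheckGamepads, which nothing in this graph calls, destroys each cached controller whose array index has no assigned gamepad.
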(event `self.ReceiveBeginPlay`
  (for _index (range (`self.MaxPlayers`))
    (set `self.Index` _index)
    (`GameplayStatics.CreatePlayer` (`self.Index`)))
  (bind _outactors (`GameplayStatics.GetAllActorsOfClass` "/Script/Engine.PlayerController"))
  (set `self.PCArray` _outactors))

(event `CheckGamepads`
  ;[1 1 1] If there are not enough gamepads, destroy excess controllers
  (for (_array_element _array_index) (`self.PCArray`)
    (if (not (`KismetSystemLibrary.IsControllerAssignedToGamepad` _array_index))
      (`self.K2_DestroyActor` _array_element))))

(fn `UserConstructionScript`)