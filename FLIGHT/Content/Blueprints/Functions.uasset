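; A set of utility functions for playing random sounds and sorting arrays.
; RandomSoundFromArray plays a randomly indexed sound at a location, with an inclusive upper bound equal to the array length, one past the last index.
; SortMinToMax bubble-sorts ascending, stopping when a pass makes no swaps, and returns the sorted array with each element's original index.
; Delegate is an empty stub.
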(fn `Delegate`)

(fn `RandomSoundFromArray`
  (params (SoundArray :type "Array of SoundWave Object Reference") (Location :type "Vector Structure"))
  (`GameplayStatics.PlaySoundAtLocation` null (`|GetArrayItem` SoundArray (`KismetMathLibrary.RandomIntegerInRange` 0 (`KismetArrayLibrary.Array_Length` SoundArray))) Location (struct) 1.0 1.0 0.0 null null null))

(fn `SortMinToMax`
  (params (UnsortedArray :type "Array of Integer"))
  (returns (SortedArray :type "Array of Integer") (`Indices of Sorted Array` :type "Array of Integer"))
  (locals (unsorted :type "Array of Integer") (Swap :type Boolean) (sortingcounter :type Integer) (Indexes :type "Array of Integer"))
  (bind _unsorted (`local.unsorted`))
  (bind _sortingcounter (`local.sortingcounter`))
  ;[1 1 1] Construct array of original indices
  (for _index (range (+ (`KismetArrayLibrary.Array_Length` UnsortedArray) 1))
    (`KismetArrayLibrary.Array_Add` (`local.Indexes`) _index))
  (set `local.unsorted` UnsortedArray)
  (for (_array_element _array_index) (`local.unsorted`) :!label _label
    (bind _returnvalue (+ _array_index 1))
    (if (`KismetArrayLibrary.Array_IsValidIndex` (`local.unsorted`) _returnvalue)
      (if (> _array_element (`|GetArrayItem` (`local.unsorted`) _returnvalue))
        ;[1 1 1] If no swaps occured this cycle, the array is "sorted"
        (`KismetArrayLibrary.Array_Swap` (`local.unsorted`) _array_index _returnvalue)
        (`KismetArrayLibrary.Array_Swap` (`local.Indexes`) _array_index _returnvalue)
        (set `local.Swap` true))))
  (if (`local.Swap`)
    (set `local.Swap` false)
    (`/Engine/EditorBlueprintResources/StandardMacros.IncrementInt` _sortingcounter
      (:`  `
        (if (>= _sortingcounter (`KismetArrayLibrary.Array_Length` _unsorted))
          _
          (else
            (goto _label))))))
  (return _unsorted (`local.Indexes`)))