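; Competitive player state that scores a player's round in what appears to be a fuel-and-landing game with payload pickups.
; CalculateRoundScore sums fuel, landing zone, time bonus and payload scores into RoundPoints.
; The fuel term adds the existing RoundPoints to remaining fuel before truncating, so earlier points carry into the new total.
; The other scores arrive precomputed and pass through unchanged; event and construction graphs are empty.
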(fn `CalculateRoundScore`
  (params (FuelRemaining :type "Float (double-precision)") (LandingZoneScore :type Integer) (TimeScore :type Integer) (PayloadScore :type Integer))
  ;[1 1 1] get 1x point for every unit of fuel remaining
  (set `self.FuelScore` (`KismetMathLibrary.FTrunc` (+ FuelRemaining (`KismetMathLibrary.Conv_IntToDouble` (`self.RoundPoints`)))))
  ;[1 1 1] Landing Zones are either 200 - 300 - 500 - or 1000 points: rated for size of landing area
  (set `self.LandingZoneScore` LandingZoneScore)
  ;[1 1 1] Time Bonus: Starts at 2000 points, decreases by 100 every for every second
  (set `self.TimeBonusScore` TimeScore)
  ;[1 1 1] Payload Score: Bonus 250 points for each unit of cargo picked up
  (set `self.PayloadScore` PayloadScore)
  (set `self.RoundPoints` (+ (`self.FuelScore`) (`self.LandingZoneScore`) (`self.TimeBonusScore`) (`self.PayloadScore`))))

(fn `UserConstructionScript`)